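; Grookey actor that blinks its right eye through a material parameter.
; BeginPlay creates dynamic material instances for the right and left eye slots of the static mesh.
; Tick writes the eye parameter, swaps its value between 0 and 1, and flips the blink flag after a half-second Delay.
; The left eye instance is created but never animated.
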(event EventBeginPlay
  (Utilities|FlowControl|Sequence
    (:then_0
      (bind _returnvalue (Rendering|Material|CreateDynamicMaterialInstance (Variables|Default|GetGrookey_StaticMesh) 1 0 "None" :!class /Script/Engine.PrimitiveComponent))
      (Variables|Default|SetREyeMaterial _returnvalue))
    (:then_1
      (bind _returnvalue_2 (Rendering|Material|CreateDynamicMaterialInstance (Variables|Default|GetGrookey_StaticMesh) 2 0 "None" :!class /Script/Engine.PrimitiveComponent))
      (Variables|Default|SetLEyeMaterial _returnvalue_2))))

(event Collision|EventActorBeginOverlap
  (params (OtherActor :type Actor%20Object%20Reference)))

(event EventTick
  (params (DeltaSeconds :type Float%20%28single-precision%29))
  (if (Variables|Default|GetIsBlink)
    (Rendering|Material|SetScalarParameterValue (Variables|Default|GetREyeMaterial) "Param_Eye_R" (Variables|Default|GetREyeParamValue) :!class /Script/Engine.MaterialInstanceDynamic)
    (Variables|Default|SetREyeParamValue 0.0)
    (Utilities|FlowControl|Delay 0.5)
    (Variables|Default|SetIsBlink false)
    (else
      (Rendering|Material|SetScalarParameterValue (Variables|Default|GetREyeMaterial) "Param_Eye_R" (Variables|Default|GetREyeParamValue) :!class /Script/Engine.MaterialInstanceDynamic)
      (Variables|Default|SetREyeParamValue 1.0)
      (Utilities|FlowControl|Delay 0.5)
      (Variables|Default|SetIsBlink true))))

(fn ConstructionScript)